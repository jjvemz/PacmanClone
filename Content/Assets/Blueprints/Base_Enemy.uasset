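; Base enemy with Pac-Man-style chase, flee and respawn behavior, driven by state flags on Tick.
; After a start delay it chases the player, or while fleeing repaths to random reachable points around the player through a timed DoOnce.
; Player overlap kills the enemy when vulnerable, otherwise the player if killable.
; A dead enemy changes color, runs to HomeBase, then revives after a rest delay and resumes chasing.
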(event OnComponentBeginOverlap(CollisionRadius)
  (params (OverlappedComponent :type Primitive%20Component%20Object%20Reference) (OtherActor :type Actor%20Object%20Reference) (OtherComp :type Primitive%20Component%20Object%20Reference) (OtherBodyIndex :type Integer) (bFromSweep :type Boolean) (SweepResult :type Hit%20Result%20Structure%20%28by%20ref%29))
  (bind _playercharacter (Variables|BlueprintReferences|GetPlayerCharacter))
  (if (== (Variables|BlueprintReferences|GetPlayerCharacter) OtherActor)
    (if (Variables|Default|GetCanCharacterDie?)
      (CallFunction|CharacterDeath)
      (elif (Variables|/Game/Assets/Blueprints/MasterCharacter.MasterCharacter_C|GetCanCharacterDie? _playercharacter)
        (Variables|/Game/Assets/Blueprints/Base_PlayerCharacter.Base_PlayerCharacter_C|SetEnemy _playercharacter self)
        (Default|CharacterDeath _playercharacter)))))

(event EventBeginPlay
  (Variables|/Script/Engine.CharacterMovementComponent|SetMaxWalkSpeed (Variables|Character|GetCharacterMovement) (Variables|Attributes|GetMaxWalkSpeed))
  (Variables|BlueprintReferences|SetEnemyController (Pawn|GetController))
  (bind _asbase_player_character (Utilities|Casting|CastToBase_PlayerCharacter (Game|GetPlayerCharacter 0)))
  (Variables|BlueprintReferences|SetPlayerCharacter _asbase_player_character)
  (Utilities|FlowControl|Delay (Variables|Attributes|GetChaseDelay))
  (Variables|Attributes|SetChaseStart? true))

(event EventTick
  (params (DeltaSeconds :type Float%20%28single-precision%29))
  (if (Variables|Attributes|GetChaseStart?)
    (if (Variables|Attributes|GetRunningFromPlayer?)
      ;[1 1 1] Movement Logic For After Power Pickup Has Been Picked Up If Enemy Is Alive
      (Utilities|FlowControl|DoOnce false :!label _label
        (:Completed
          (AI|AIMoveTo self (.RandomLocation (AI|Navigation|GetRandomReachablePointinRadius (Transformation|GetActorLocation (Variables|BlueprintReferences|GetPlayerCharacter)) 1e+04 0 0)) 0 1e+02 false
            (:then
              _)
            (:OnSuccess
              _)
            (:OnFail
              _))
          (Utilities|FlowControl|Delay (Math|Random|RandomFloatinRange 0.5 2.0))
          (goto _label Reset)))
      (elif (Variables|Attributes|GetChasingPlayer?)
        ;[1 0 0] Normal Movement Logic
        (AI|Navigation|SimpleMovetoActor (Variables|BlueprintReferences|GetEnemyController) (Variables|BlueprintReferences|GetPlayerCharacter))
        (elif (Math|Vector|Equal(Vector) (Transformation|GetActorLocation) (Transformation|GetActorLocation (Variables|Attributes|GetHomeBase)) 1e+02)
          ;[0 0 0.6719] After Enemy Has Been Killed, And Is At Home Base, Recover for Rest Delay Amount Then Come Back Alive
          (Utilities|FlowControl|Delay (Variables|Attributes|GetRestDelay))
          (Variables|Default|SetIsCharacterAlive? true)
          (Variables|Default|SetCanCharacterDie? false)
          (Variables|Attributes|SetChasingPlayer? true)
          (CallFunction|ChangeColors (Variables|Default|GetColor))
          (else
            ;[0 0 0.6719] After Enemy Has Been Killed, Run To Home Base Movement Logic
            (AI|Navigation|SimpleMovetoActor (Variables|BlueprintReferences|GetEnemyController) (Variables|Attributes|GetHomeBase))))))))

(event EventCharacterDeath
  (Variables|Default|SetIsCharacterAlive? false)
  (Variables|Attributes|SetRunningFromPlayer? false)
  (Variables|Attributes|SetChasingPlayer? false)
  (CallFunction|ChangeColors "(R=0.019608,G=0.019608,B=0.835294,A=1.000000)"))

(fn ConstructionScript
  (|CallParentFunction))