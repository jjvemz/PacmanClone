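; Base geometry Blueprint that serves as either a floor or a wall piece, chosen by its TypeOfGeometry value.
; The construction script switches on that value, assigning a plane mesh for floors or a one-metre cube for walls, then calls the parent script.
; Walls also get their mesh component raised by a world-space offset of half a metre.
; The event graph holds only disabled default events, so it adds no runtime logic.
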(event EventBeginPlay
  (|CallParentFunction) ; This node is disabled and will not be called.\nDrag off pins to build functionality.
)

(event Collision|EventActorBeginOverlap
  (params (OtherActor :type Actor%20Object%20Reference))
  (|CallParentFunction OtherActor) ; This node is disabled and will not be called.\nDrag off pins to build functionality.
)

(event EventTick
  (params (DeltaSeconds :type Float%20%28single-precision%29))
  (|CallParentFunction DeltaSeconds) ; This node is disabled and will not be called.\nDrag off pins to build functionality.
)

(fn ConstructionScript
  (bind _staticmesh (Variables|Default|GetStaticMesh))
  (switch Utilities|FlowControl|Switch|SwitchonGeometryType (Variables|Default|GetTypeOfGeometry)
    (:NewEnumerator0
      (Components|StaticMesh|SetStaticMesh (Variables|Default|GetStaticMesh) "/Game/Assets/Shapes/Shape_Plane.Shape_Plane"))
    (:NewEnumerator1
      (Components|StaticMesh|SetStaticMesh _staticmesh "/Game/Geometry/Meshes/1M_Cube.1M_Cube")
      (Transformation|AddWorldOffset _staticmesh "0, 0,50.000000" false false)))
  (|CallParentFunction))