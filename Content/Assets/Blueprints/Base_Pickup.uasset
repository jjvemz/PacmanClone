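; Base pickup actor that the player character collects on contact, in either a Dot or Power variant.
; On overlap with its pickup radius, it casts to Base_PlayerCharacter, increments that player's count for its type, and destroys itself.
; Power pickups also trigger the player's CollectedPowerPickup, and the construction script rescales their static mesh to set them apart.
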(event OnComponentBeginOverlap(PickupRadius)
  (params (OverlappedComponent :type Primitive%20Component%20Object%20Reference) (OtherActor :type Actor%20Object%20Reference) (OtherComp :type Primitive%20Component%20Object%20Reference) (OtherBodyIndex :type Integer) (bFromSweep :type Boolean) (SweepResult :type Hit%20Result%20Structure%20%28by%20ref%29))
  (bind _pickuptype (Variables|Default|GetPickupType))
  (bind _asbase_player_character (Utilities|Casting|CastToBase_PlayerCharacter OtherActor))
  (bind _output_get (Variables|Default|SetPlayerReference _asbase_player_character))
  (Default|IncreaseCount _output_get _pickuptype)
  (switch Utilities|FlowControl|Switch|SwitchonPickupType _pickuptype
    (:NewEnumerator0
      _)
    (:NewEnumerator1
      (Default|CollectedPowerPickup (Variables|Default|GetPlayerReference))))
  (Utilities|IsValid self
    (:Is%20Valid
      (Actor|DestroyActor))))

(event EventBeginPlay
  (|CallParentFunction) ; This node is disabled and will not be called.\nDrag off pins to build functionality.
)

(event Collision|EventActorBeginOverlap
  (params (OtherActor :type Actor%20Object%20Reference))
  (|CallParentFunction OtherActor) ; This node is disabled and will not be called.\nDrag off pins to build functionality.
)

(event EventTick
  (params (DeltaSeconds :type Float%20%28single-precision%29))
  (|CallParentFunction DeltaSeconds) ; This node is disabled and will not be called.\nDrag off pins to build functionality.
)

(fn ConstructionScript
  (switch Utilities|FlowControl|Switch|SwitchonPickupType (Variables|Default|GetPickupType)
    (:NewEnumerator0
      _)
    (:NewEnumerator1
      (Transformation|SetWorldScale3D (Variables|Default|GetStaticMesh) "0.500000,0.500000,0.500000")))
  (|CallParentFunction))